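; BP_Pillar_Of_Fire_Projectile is a pillar of fire weapon projectile that deals repeated area damage to enemies overlapping it.
; BeginPlay starts DamageWithin, a self-calling event that applies the Damage value to each overlapping BP_Enemy_Base_Class actor, then repeats after a short Delay.
; Damage comes from this polling loop rather than overlap events, so enemies are hit continuously while they stay inside.
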(event Custom|DamageWithin
  (for _array_element (Collision|GetOverlappingActors "/Game/Dynasty/Enemies/BP_Enemy_Base_Class.BP_Enemy_Base_Class_C" :!class /Script/Engine.Actor)
    (bind _asbp_enemy_base_class (Utilities|Casting|CastToBP_Enemy_Base_Class _array_element))
    (CallFunction|ApplyDamage _asbp_enemy_base_class (Variables|Default|GetDamage)))
  (Utilities|FlowControl|Delay 0.1)
  (CallFunction|DamageWithin))

(event EventBeginPlay
  (CallFunction|DamageWithin))

(event Collision|EventActorBeginOverlap
  (params (OtherActor :type Actor%20Object%20Reference)))

(event EventTick
  (params (DeltaSeconds :type Float%20%28single-precision%29)))

(fn ConstructionScript
  (|CallParentFunction))