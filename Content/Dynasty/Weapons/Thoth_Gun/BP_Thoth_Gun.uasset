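; Thoth Gun weapon Blueprint that fires a BP_ThothProj projectile when Shoot is called.
; Shoot spawns it at the location and rotation of the first-person character's ProjOrigin, ignoring its start and end location inputs.
; Disconnected old ray-cast code remains, which placed a ground-traced pillar of fire, scaled up by the Flame Dispersion flag.
; The event graph is empty, and construction only calls the parent script.
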(event EventBeginPlay)

(event Collision|EventActorBeginOverlap
  (params (OtherActor :type Actor%20Object%20Reference)))

(event EventTick
  (params (DeltaSeconds :type Float%20%28single-precision%29)))

(fn ConstructionScript
  (|CallParentFunction))

(fn Shoot
  (params (StartLocation :type Vector :default "0, 0, 0") (EndLocation :type Vector :default "0, 0, 0"))
  (bind _firstpersoncharacterreference (Variables|Default|GetFirstPersonCharacterReference))
  (bind _projorigin (Variables|/Game/FirstPerson/Blueprints/BP_FirstPersonCharacter.BP_FirstPersonCharacter_C|GetProjOrigin _firstpersoncharacterreference))
  (bind _returnvalue (Transformation|GetWorldTransform _projorigin))
  (Game|SpawnActorfromClass "/Game/Dynasty/Weapons/Thoth_Gun/BP_ThothProj.BP_ThothProj_C" (Math|Transform|MakeTransform (.location _returnvalue) (.rotation _returnvalue) "1.000000,1.000000,1.000000") "Undefined" "MultiplyWithRoot" 0 0))