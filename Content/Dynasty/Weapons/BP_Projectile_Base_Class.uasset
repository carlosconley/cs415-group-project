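; Base projectile Blueprint for weapons that provides shared damage functions scaled by the first-person player character's upgrades.
; ApplyDamage flags enemies as blaze-crippled or starts their one-time germinating spore damage event when the player has those effects, then deals damage times DamageMultiplier.
; ApplyDamagePlayer handles self-damage, scaling it by both DamageMultiplier and DamageTakenFactor.
; Both functions read these values from player 0's character.
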(fn ConstructionScript)

(fn ApplyDamage
  (params (Enemy :type BP%20Enemy%20Base%20Class%20Object%20Reference) (Damage :type Float%20%28double-precision%29))
  (bind _asbp_first_person_character (Utilities|Casting|CastToBP_FirstPersonCharacter (Game|GetPlayerCharacter 0)))
  (Utilities|FlowControl|Sequence
    (:then_0
      (if (Variables|/Game/FirstPerson/Blueprints/BP_FirstPersonCharacter.BP_FirstPersonCharacter_C|GetHasCripplingBlaze _asbp_first_person_character)
        (Variables|/Game/Dynasty/Enemies/BP_Enemy_Base_Class.BP_Enemy_Base_Class_C|SetIsBlazeCrippled Enemy true)))
    (:then_1
      (if (Variables|/Game/FirstPerson/Blueprints/BP_FirstPersonCharacter.BP_FirstPersonCharacter_C|GetHasGerminatingSpores _asbp_first_person_character)
        ;[1 1 1] Begin the germinating spore damage event only once
        (if (not (Variables|/Game/Dynasty/Enemies/BP_Enemy_Base_Class.BP_Enemy_Base_Class_C|GetIsGerminatingSpored Enemy))
          (Variables|/Game/Dynasty/Enemies/BP_Enemy_Base_Class.BP_Enemy_Base_Class_C|SetIsGerminatingSpored Enemy true)
          (Default|TakeGerminatingSporeDamage Enemy))))
    (:then_2
      (Game|Damage|ApplyDamage Enemy (* Damage (Variables|/Game/FirstPerson/Blueprints/BP_FirstPersonCharacter.BP_FirstPersonCharacter_C|GetDamageMultiplier _asbp_first_person_character)) 0 0))))

(fn ApplyDamagePlayer
  (params (Damage :type Float%20%28double-precision%29))
  ;[1 1 1] For applying damage to self
  (bind _asbp_first_person_character (Utilities|Casting|CastToBP_FirstPersonCharacter (Game|GetPlayerCharacter 0)))
  (Game|Damage|ApplyDamage _asbp_first_person_character (* Damage (Variables|/Game/FirstPerson/Blueprints/BP_FirstPersonCharacter.BP_FirstPersonCharacter_C|GetDamageMultiplier _asbp_first_person_character) (Variables|/Game/FirstPerson/Blueprints/BP_FirstPersonCharacter.BP_FirstPersonCharacter_C|GetDamageTakenFactor _asbp_first_person_character)) 0 0))