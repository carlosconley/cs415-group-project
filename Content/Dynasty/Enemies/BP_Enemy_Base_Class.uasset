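; Base enemy class that handles damage, death and reporting to the room that owns the enemy.
; Any damage is scaled by the first-person player's DamageMultiplier, whatever the source, then subtracted from Health.
; At zero Health, OnDeath notifies OwningRoom via CheckDeath, and Dying stops AI logic, plays the death animation and destroys the actor after a delay.
; Only Dying is guarded against repeats, so further hits call OnDeath again.
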(event Custom|Dying
  (if (not (Variables|Default|GetInDying))
    (Variables|Default|SetInDying true)
    (AI|Logic|StopLogic (Variables|/Script/AIModule.AIController|GetBrainComponent (AI|GetAIController self)) "")
    (Components|Animation|PlayAnimation (Variables|Character|GetMesh) (Variables|Default|GetDeathAnimation) false)
    (Utilities|FlowControl|Delay 2.0)
    (Actor|DestroyActor)))

(event EventBeginPlay)

(event Collision|EventActorBeginOverlap
  (params (OtherActor :type Actor%20Object%20Reference)))

(event EventTick
  (params (DeltaSeconds :type Float%20%28single-precision%29)))

(event Game|Damage|EventAnyDamage
  (params (Damage :type Float%20%28single-precision%29) (DamageType :type Damage%20Type%20Object%20Reference) (InstigatedBy :type Controller%20Object%20Reference) (DamageCauser :type Actor%20Object%20Reference))
  (bind _asbp_first_person_character (Utilities|Casting|CastToBP_FirstPersonCharacter (Game|GetPlayerCharacter 0)))
  (bind _output_get (Variables|Default|SetHealth (- (Variables|Default|GetHealth) (* (Variables|/Game/FirstPerson/Blueprints/BP_FirstPersonCharacter.BP_FirstPersonCharacter_C|GetDamageMultiplier _asbp_first_person_character) Damage))))
  (bind _output_get_2 (Variables|Default|SetIsDead (<= _output_get 0.0)))
  (if _output_get_2
    (CallFunction|OnDeath)
    (CallFunction|Dying)))

(fn ConstructionScript)

(fn OnDeath
  (bind _owningroom (Variables|Default|GetOwningRoom))
  (Variables|Default|SetIsDead true)
  (Utilities|IsValid _owningroom
    (:Is%20Valid
      (Default|CheckDeath _owningroom)
      (Development|PrintString "Enemy died"))))