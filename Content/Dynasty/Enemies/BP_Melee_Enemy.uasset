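; BP_Melee_Enemy is a melee enemy that damages the first-person player character through mesh overlap.
; MeleeAttack enables attack detection and plays a random animation from the Animations array on the mesh.
; While detection is on, mesh overlaps with BP_FirstPersonCharacter apply fixed damage and print a debug message; nothing here switches detection off.
; UpdateWalkSpeed sets the character movement's maximum walk speed.
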(event OnComponentBeginOverlap(Mesh)
  (params (OverlappedComponent :type Primitive%20Component%20Object%20Reference) (OtherActor :type Actor%20Object%20Reference) (OtherComp :type Primitive%20Component%20Object%20Reference) (OtherBodyIndex :type Integer) (bFromSweep :type Boolean) (SweepResult :type Hit%20Result%20Structure%20%28by%20ref%29))
  (if (Variables|Default|GetShouldDetectAttack)
    (bind _asbp_first_person_character (Utilities|Casting|CastToBP_FirstPersonCharacter OtherActor))
    (Game|Damage|ApplyDamage _asbp_first_person_character 1e+01 0 0)
    (Development|PrintString "Doing Damage")))

(event Custom|MeleeAttack
  (Variables|Default|SetShouldDetectAttack (Math|Conversions|ToBoolean(Integer) 1))
  (Components|Animation|PlayAnimation (Variables|Character|GetMesh) (.OutItem (Utilities|Array|Random (Variables|Default|GetAnimations))) false))

(event EventBeginPlay)

(event Collision|EventActorBeginOverlap
  (params (OtherActor :type Actor%20Object%20Reference)))

(event EventTick
  (params (DeltaSeconds :type Float%20%28single-precision%29)))

(fn ConstructionScript
  (|CallParentFunction))

(fn UpdateWalkSpeed
  (params (NewWalkSpeed :type Float%20%28double-precision%29))
  (Variables|/Script/Engine.CharacterMovementComponent|SetMaxWalkSpeed (Variables|Character|GetCharacterMovement) NewWalkSpeed))