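; BP_Ranged_Enemy is a ranged enemy that carries a crossbow and shoots arrows at the player.
; On BeginPlay it spawns a non-colliding crossbow attached to the GripPoint socket, and destroys it when the enemy is destroyed.
; RangeAttack plays the shoot animation and immediately spawns an arrow ahead of the grip bone, rotated toward the player character.
; The construction script records the actor's spawn location.
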(event Custom|RangeAttack
  (Components|Animation|PlayAnimation (Variables|Character|GetMesh) "/Game/Dynasty/Enemies/Assets/SkeletonRogue/Skeleton_Rogue_Anim_1H_Ranged_Shoot.Skeleton_Rogue_Anim_1H_Ranged_Shoot" false)
  (CallFunction|SpawnArrow))

(event Custom|Death
  (params (DestroyedActor :type Actor%20Object%20Reference))
  (Actor|DestroyActor (Variables|Default|GetCrossbow)))

(event Collision|EventActorBeginOverlap
  (params (OtherActor :type Actor%20Object%20Reference))
  (|CallParentFunction OtherActor) ; This node is disabled and will not be called.\nDrag off pins to build functionality.
)

(event EventTick
  (params (DeltaSeconds :type Float%20%28single-precision%29))
  (|CallParentFunction DeltaSeconds) ; This node is disabled and will not be called.\nDrag off pins to build functionality.
)

(event EventBeginPlay
  (bind _returnvalue (Game|SpawnActorfromClass "/Game/Dynasty/Enemies/Assets/Weapons/Crossbow.Crossbow_C" (Math|Transform|MakeTransform "0, 0, 0" "0, 0, 0" "1.000000,1.000000,1.000000") "Undefined" "MultiplyWithRoot" 0 0))
  (bind _output_get (Variables|Default|SetCrossbow _returnvalue))
  (Collision|SetCollisionEnabled (Variables|/Game/Dynasty/Enemies/Assets/Weapons/Crossbow.Crossbow_C|GetStaticMesh _output_get) "NoCollision")
  (Transformation|AttachComponentToComponent _returnvalue (Variables|Character|GetMesh) "GripPoint" "KeepRelative" "KeepRelative" "KeepRelative" true)
  (EventDispatchers|BindEventtoOnDestroyed (delegate Custom|Death)))

(fn ConstructionScript
  (|CallParentFunction)
  (Variables|Default|SetSpawnLocation (Transformation|GetActorLocation)))

(fn SpawnArrow
  (bind _mesh (Variables|Character|GetMesh))
  (bind _returnvalue (Class|SkinnedMeshComponent|GetSocketBoneName _mesh "GripPoint"))
  (bind _returnvalue_2 (Transformation|GetSocketLocation _mesh _returnvalue))
  (Game|SpawnActorfromClass "/Game/Dynasty/Enemies/RangedEnemy/BP_Ranged_Enemy_Arrow.BP_Ranged_Enemy_Arrow_C" (Math|Transform|MakeTransform (+ _returnvalue_2 (* (Transformation|GetActorForwardVector) "50.000000,50.000000,50.000000")) (Math|Conversions|RotationFromXVector (- (Transformation|GetActorLocation (Game|GetPlayerCharacter 0)) _returnvalue_2)) "1.000000,1.000000,1.000000") "Undefined" "MultiplyWithRoot" 0 0))