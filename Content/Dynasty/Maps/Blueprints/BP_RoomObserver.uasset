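; Room observer owned by a BP_Door that opens that door once all enemies are dead.
; On BeginPlay it gathers every BP_Enemy_Base_Class actor in the world, registers itself as each one's OwningRoom, and caches its owner as the door inside that loop.
; CheckDeath, which has no caller in this Blueprint, scans for living enemies and, finding none, marks the level complete and triggers the door's open event.
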(event EventBeginPlay
  (bind _outactors (Actor|GetAllActorsOfClass "/Game/Dynasty/Enemies/BP_Enemy_Base_Class.BP_Enemy_Base_Class_C"))
  (bind _output_get (Variables|Default|SetEnemies _outactors))
  (for _array_element _output_get
    (Variables|/Game/Dynasty/Enemies/BP_Enemy_Base_Class.BP_Enemy_Base_Class_C|SetOwningRoom _array_element self)
    (bind _asbp_door (Utilities|Casting|CastToBP_Door (Components|GetOwner))
      (:then
        (Variables|Default|SetLevelDoor _asbp_door))
      (:CastFailed
        (Development|PrintString "COULD NOT FIND DOOR")))))

(event EventTick
  (params (DeltaSeconds :type Float%20%28single-precision%29)))

(fn CheckDeath
  (bind _array_element (Utilities|Array|ForEachLoopwithBreak (Variables|Default|GetEnemies) :!label _label)
    (:LoopBody
      (if (Utilities|IsValid _array_element)
        (if (not (Variables|/Game/Dynasty/Enemies/BP_Enemy_Base_Class.BP_Enemy_Base_Class_C|GetIsDead _array_element))
          (LocalVariables|SetAllDead false)
          (goto _label Break))))
    (:Completed
      (if (LocalVariables|GetAllDead)
        ;[1 1 1] if true open door
        (Variables|Default|SetIsLevelComplete true)
        (Default|EventOpenDoor (Variables|Default|GetLevelDoor))))))