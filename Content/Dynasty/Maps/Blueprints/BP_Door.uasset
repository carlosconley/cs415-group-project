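; BP_Door is a level exit door that lets the first-person player advance or win once it has been opened.
; OpenDoor marks it open and swaps the cube's material.
; Overlapping its box while open saves player info to PlayerInstance and loads NextLevel.
; If flagged as the final door, it instead shows the win screen, pauses with UI-only input and disables save loading.
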(event OnComponentBeginOverlap(Box)
  (params (OverlappedComponent :type Primitive%20Component%20Object%20Reference) (OtherActor :type Actor%20Object%20Reference) (OtherComp :type Primitive%20Component%20Object%20Reference) (OtherBodyIndex :type Integer) (bFromSweep :type Boolean) (SweepResult :type Hit%20Result%20Structure%20%28by%20ref%29))
  (bind _returnvalue (Game|GetPlayerController 0))
  (bind _asbp_first_person_character (Utilities|Casting|CastToBP_FirstPersonCharacter OtherActor))
  (if (Variables|Default|GetIsOpen)
    (if (Variables|Default|GetIsFinalDoor)
      (Variables|/Script/Engine.PlayerController|SetbShowMouseCursor _returnvalue true)
      (Input|SetInputModeUIOnly _returnvalue 0 "DoNotLock" true)
      (Default|ShowWinScreen (Variables|/Game/FirstPerson/Blueprints/BP_FirstPersonCharacter.BP_FirstPersonCharacter_C|GetHUD _asbp_first_person_character))
      (Game|SetGamePaused true)
      (Variables|/Game/FirstPerson/Blueprints/GI_DynastyGameInstance.GI_DynastyGameInstance_C|SetShouldLoad (Variables|/Game/FirstPerson/Blueprints/BP_FirstPersonCharacter.BP_FirstPersonCharacter_C|GetPlayerInstance _asbp_first_person_character) false)
      (else
        (Default|UpdatePlayerInfo (Variables|/Game/FirstPerson/Blueprints/BP_FirstPersonCharacter.BP_FirstPersonCharacter_C|GetPlayerInstance _asbp_first_person_character) _asbp_first_person_character)
        (Game|OpenLevel(byName) (Variables|Default|GetNextLevel))))))

(event Custom|Event%20Open%20Door
  (Variables|Default|SetIsOpen true)
  (Rendering|Material|SetMaterial (Variables|Default|GetSM_Cube) 0 "/Engine/VREditor/BasicMeshes/MI_Pyramid_01.MI_Pyramid_01"))

(event EventBeginPlay)

(event EventTick
  (params (DeltaSeconds :type Float%20%28single-precision%29)))

(fn ConstructionScript)