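; Pharaoh's Grandeur is an upgrade from the Osiris set that trades movement speed for shorter weapon cooldowns.
; On pickup it flags the owning player as having the upgrade and halves both the movespeed and weapon cooldown multipliers, then calls the parent pickup logic.
; The multipliers are scaled from their current values, so the effect compounds with other modifiers.
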(event EventBeginPlay
  (|CallParentFunction) ; This node is disabled and will not be called.\nDrag off pins to build functionality.
)

(event EventTick
  (params (DeltaSeconds :type Float%20%28single-precision%29))
  (|CallParentFunction DeltaSeconds) ; This node is disabled and will not be called.\nDrag off pins to build functionality.
)

(fn OnPickup
  (params (OwningPlayer :type BP%20First%20Person%20Character%20Object%20Reference))
  (Variables|/Game/FirstPerson/Blueprints/BP_FirstPersonCharacter.BP_FirstPersonCharacter_C|SetHasPharaohsGrandeur OwningPlayer true)
  (Variables|/Game/FirstPerson/Blueprints/BP_FirstPersonCharacter.BP_FirstPersonCharacter_C|SetMovespeedMultiplier OwningPlayer (* (Variables|/Game/FirstPerson/Blueprints/BP_FirstPersonCharacter.BP_FirstPersonCharacter_C|GetMovespeedMultiplier OwningPlayer) 0.5))
  (Variables|/Game/FirstPerson/Blueprints/BP_FirstPersonCharacter.BP_FirstPersonCharacter_C|SetWeaponCooldownMultiplier OwningPlayer (* 0.5 (Variables|/Game/FirstPerson/Blueprints/BP_FirstPersonCharacter.BP_FirstPersonCharacter_C|GetWeaponCooldownMultiplier OwningPlayer)))
  (|CallParentFunction OwningPlayer))