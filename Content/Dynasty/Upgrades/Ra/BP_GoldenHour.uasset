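; BP_GoldenHour is a Ra upgrade that trades a player's maximum health for shields when picked up.
; OnPickup flags the player as having Golden Hour, scales the health multiplier multiplicatively rather than additively, then updates max health.
; It converts the resulting drop in max health into shields through a conversion factor before calling the parent pickup logic.
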(event EventBeginPlay
  (|CallParentFunction) ; This node is disabled and will not be called.\nDrag off pins to build functionality.
)

(event EventTick
  (params (DeltaSeconds :type Float%20%28single-precision%29))
  (|CallParentFunction DeltaSeconds) ; This node is disabled and will not be called.\nDrag off pins to build functionality.
)

(fn OnPickup
  (params (OwningPlayer :type BP%20First%20Person%20Character%20Object%20Reference))
  (Variables|/Game/FirstPerson/Blueprints/BP_FirstPersonCharacter.BP_FirstPersonCharacter_C|SetHasGoldenHour OwningPlayer true)
  (LocalVariables|SetPreviousMaxHP (Variables|/Game/FirstPerson/Blueprints/BP_FirstPersonCharacter.BP_FirstPersonCharacter_C|GetMaxHealth OwningPlayer))
  (Variables|/Game/FirstPerson/Blueprints/BP_FirstPersonCharacter.BP_FirstPersonCharacter_C|SetHealthMultiplier OwningPlayer (* (Variables|Default|GetMaxHPLostFactor) (Variables|/Game/FirstPerson/Blueprints/BP_FirstPersonCharacter.BP_FirstPersonCharacter_C|GetHealthMultiplier OwningPlayer)))
  (Default|UpdateMaxHealth OwningPlayer)
  (Variables|/Game/FirstPerson/Blueprints/BP_FirstPersonCharacter.BP_FirstPersonCharacter_C|SetShields OwningPlayer (+ (Variables|/Game/FirstPerson/Blueprints/BP_FirstPersonCharacter.BP_FirstPersonCharacter_C|GetShields OwningPlayer) (* (Variables|Default|GetShieldConversionFactor) (- (LocalVariables|GetPreviousMaxHP) (Variables|/Game/FirstPerson/Blueprints/BP_FirstPersonCharacter.BP_FirstPersonCharacter_C|GetMaxHealth OwningPlayer)))))
  (|CallParentFunction OwningPlayer))