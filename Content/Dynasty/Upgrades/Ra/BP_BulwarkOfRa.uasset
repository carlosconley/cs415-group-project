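; BP_BulwarkOfRa is a Ra upgrade that modifies the owning player's health and movespeed multipliers on pickup.
; OnPickup computes the new-to-old health multiplier ratio first, then adds HealthModifyFactor, updates max health and scales current HP by that ratio to keep it proportional.
; It then calls the parent pickup logic and adds MovespeedModifyFactor to the movespeed multiplier.
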(event EventBeginPlay
  (|CallParentFunction) ; This node is disabled and will not be called.\nDrag off pins to build functionality.
)

(event EventTick
  (params (DeltaSeconds :type Float%20%28single-precision%29))
  (|CallParentFunction DeltaSeconds) ; This node is disabled and will not be called.\nDrag off pins to build functionality.
)

(fn OnPickup
  (params (OwningPlayer :type BP%20First%20Person%20Character%20Object%20Reference))
  (Utilities|FlowControl|Sequence
    (:then_0
      ;[1 1 1] Compute Ratio of New to Old Health
      (LocalVariables|SetHP_RatioNewVsOld (/ (+ (Variables|/Game/FirstPerson/Blueprints/BP_FirstPersonCharacter.BP_FirstPersonCharacter_C|GetHealthMultiplier OwningPlayer) (Variables|Default|GetHealthModifyFactor)) (Variables|/Game/FirstPerson/Blueprints/BP_FirstPersonCharacter.BP_FirstPersonCharacter_C|GetHealthMultiplier OwningPlayer))))
    (:then_1
      (Variables|/Game/FirstPerson/Blueprints/BP_FirstPersonCharacter.BP_FirstPersonCharacter_C|SetHealthMultiplier OwningPlayer (+ (Variables|/Game/FirstPerson/Blueprints/BP_FirstPersonCharacter.BP_FirstPersonCharacter_C|GetHealthMultiplier OwningPlayer) (Variables|Default|GetHealthModifyFactor)))
      (Default|UpdateMaxHealth OwningPlayer)
      ;[1 1 1] Also Update Current HP by the Same Factor as Max HP Change
      (Default|UpdateHealth OwningPlayer (* (Variables|/Game/FirstPerson/Blueprints/BP_FirstPersonCharacter.BP_FirstPersonCharacter_C|GetHealth OwningPlayer) (LocalVariables|GetHP_RatioNewVsOld)))
      (|CallParentFunction 0))
    (:then_2
      (Variables|/Game/FirstPerson/Blueprints/BP_FirstPersonCharacter.BP_FirstPersonCharacter_C|SetMovespeedMultiplier OwningPlayer (+ (Variables|/Game/FirstPerson/Blueprints/BP_FirstPersonCharacter.BP_FirstPersonCharacter_C|GetMovespeedMultiplier OwningPlayer) (Variables|Default|GetMovespeedModifyFactor))))))