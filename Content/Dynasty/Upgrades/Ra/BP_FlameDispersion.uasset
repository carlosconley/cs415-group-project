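; BP_FlameDispersion is a pickup upgrade in the Ra dynasty set that boosts the player's maximum health.
; On pickup it adds its health buff to the player's health multiplier, then has the player recalculate max health before calling the parent pickup logic.
; Debug prints show the new multiplier and confirm the pickup; BeginPlay and Tick are unused.
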(event EventBeginPlay
  (|CallParentFunction) ; This node is disabled and will not be called.\nDrag off pins to build functionality.
)

(event EventTick
  (params (DeltaSeconds :type Float%20%28single-precision%29))
  (|CallParentFunction DeltaSeconds) ; This node is disabled and will not be called.\nDrag off pins to build functionality.
)

(fn OnPickup
  (params (OwningPlayer :type BP%20First%20Person%20Character%20Object%20Reference))
  (bind _output_get (Variables|/Game/FirstPerson/Blueprints/BP_FirstPersonCharacter.BP_FirstPersonCharacter_C|SetHealthMultiplier OwningPlayer (+ (Variables|Default|GetHealthBuffMul) (Variables|/Game/FirstPerson/Blueprints/BP_FirstPersonCharacter.BP_FirstPersonCharacter_C|GetHealthMultiplier OwningPlayer))))
  (Development|PrintString (Utilities|String|ToString(Float) _output_get) true true "(R=0.000000,G=0.660000,B=1.000000,A=1.000000)" _output_get)
  (Default|UpdateMaxHealth OwningPlayer)
  (Development|PrintString "Picked up upgrade 4")
  (|CallParentFunction OwningPlayer))