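; Osiris Orb projectile for an ability, whose damage grows with time in flight, scaled by DamageMul.
; On overlap, it applies that damage to enemies and changes the owning player's health by the negated damage times HealMul.
; It then destroys itself whether or not it hit an enemy.
; The projectile-class check guarding the overlap has no object input wired, so it filters nothing.
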(event OnComponentBeginOverlap(Collision)
  (params (OverlappedComponent :type Primitive%20Component%20Object%20Reference) (OtherActor :type Actor%20Object%20Reference) (OtherComp :type Primitive%20Component%20Object%20Reference) (OtherBodyIndex :type Integer) (bFromSweep :type Boolean) (SweepResult :type Hit%20Result%20Structure%20%28by%20ref%29))
  (bind _damage (Variables|Default|GetDamage))
  (bind _owningplayer (Variables|Default|GetOwningPlayer))
  (if (not (Class|GameplayStatics|ObjectIsA 0 "/Game/Dynasty/Weapons/BP_Projectile_Base_Class.BP_Projectile_Base_Class_C"))
    (bind _asbp_enemy_base_class (Utilities|Casting|CastToBP_Enemy_Base_Class OtherActor)
      (:then
        (Game|Damage|ApplyDamage _asbp_enemy_base_class _damage 0 0)
        (Default|UpdateHealth _owningplayer (+ (Variables|/Game/FirstPerson/Blueprints/BP_FirstPersonCharacter.BP_FirstPersonCharacter_C|GetHealth _owningplayer) (* (- 0.0 _damage) (Variables|Default|GetHealMul)))))
      (:CastFailed
        _))
    (Actor|DestroyActor)))

(event EventBeginPlay)

(event Collision|EventActorBeginOverlap
  (params (OtherActor :type Actor%20Object%20Reference)))

(event EventTick
  (params (DeltaSeconds :type Float%20%28single-precision%29))
  (Variables|Default|SetDamage (+ (* DeltaSeconds (Variables|Default|GetDamageMul)) (Variables|Default|GetDamage))))

(fn ConstructionScript)