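; BP_OsirisOrb is the Osiris Orb ability, which fires an orb projectile from the owning player.
; When activation is allowed, it spawns a BP_OsirisOrbProj at the player's ProjOrigin transform and passes the owning player to it.
; It then calls the parent ActivateAbility, which runs only on a successful activation; BeginPlay and Tick just defer to the parent.
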(event EventBeginPlay
  (|CallParentFunction))

(event EventTick
  (params (DeltaSeconds :type Float%20%28single-precision%29))
  (|CallParentFunction DeltaSeconds))

(fn ActivateAbility
  (if (Variables|Default|GetCanActivate)
    (bind _returnvalue (Game|SpawnActorfromClass "/Game/Dynasty/Abilities/OsirisOrb/BP_OsirisOrbProj.BP_OsirisOrbProj_C" (Math|Transform|MakeTransform (.location (Transformation|GetWorldTransform (Variables|/Game/FirstPerson/Blueprints/BP_FirstPersonCharacter.BP_FirstPersonCharacter_C|GetProjOrigin (Variables|Default|GetOwningPlayer)))) (.rotation (Transformation|GetWorldTransform (Variables|/Game/FirstPerson/Blueprints/BP_FirstPersonCharacter.BP_FirstPersonCharacter_C|GetProjOrigin (Variables|Default|GetOwningPlayer)))) "1.000000,1.000000,1.000000") "Undefined" "MultiplyWithRoot" 0 0))
    (Variables|/Game/Dynasty/Abilities/OsirisOrb/BP_OsirisOrbProj.BP_OsirisOrbProj_C|SetOwningPlayer _returnvalue (Variables|Default|GetOwningPlayer))
    (|CallParentFunction)))