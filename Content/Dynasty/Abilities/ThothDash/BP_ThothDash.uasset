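; BP_ThothDash is a dash ability Blueprint for Thoth that launches the owning player forward with a slight upward lift.
; It overrides ActivateAbility and, when CanActivate is true, calls LaunchCharacter along the actor's horizontal forward vector plus an up component, adding to existing velocity.
; It then calls the parent ActivateAbility, only on that successful path; BeginPlay and Tick are unused.
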(event EventBeginPlay
  (|CallParentFunction) ; This node is disabled and will not be called.\nDrag off pins to build functionality.
)

(event EventTick
  (params (DeltaSeconds :type Float%20%28single-precision%29))
  (|CallParentFunction DeltaSeconds) ; This node is disabled and will not be called.\nDrag off pins to build functionality.
)

(fn ActivateAbility
  (bind _owningplayer (Variables|Default|GetOwningPlayer))
  (if (Variables|Default|GetCanActivate)
    (Character|LaunchCharacter _owningplayer (+ (* (Transformation|GetActorForwardVector _owningplayer) "1000.000000,1000.000000,0.000000") (* (Math|Vector|GetUpVector (Transformation|GetActorRotation _owningplayer)) "0.000000,0.000000,200.000000")) false false)
    (|CallParentFunction)))