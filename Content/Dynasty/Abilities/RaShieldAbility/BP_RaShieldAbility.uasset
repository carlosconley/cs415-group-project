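; BP_RaShieldAbility is a player ability that spawns a temporary Ra shield in front of the owning player.
; ActivateAbility checks CanActivate, then fires SpawnShield and calls the parent implementation.
; SpawnShield places BP_RaShield along the player's forward vector, turned to the controller's yaw, and blocks reactivation.
; A single CoolDown delay sets both shield lifetime and lockout, after which the shield is destroyed and the ability re-enabled.
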(event Custom|Spawn%20Shield
  (bind _owningplayer (Variables|Default|GetOwningPlayer))
  (bind _returnvalue (Game|SpawnActorfromClass "/Game/Dynasty/Abilities/RaShieldAbility/BP_RaShield.BP_RaShield_C" (Math|Transform|MakeTransform (+ (Transformation|GetActorLocation _owningplayer) (* (Transformation|GetActorForwardVector _owningplayer) "100.000000,100.000000,100.000000")) (Math|Rotator|MakeRotator 0.0 0.0 (.yaw (Pawn|GetControlRotation (Game|GetPlayerController (Variables|/Script/Engine.Pawn|GetPlayerState _owningplayer)) :!class /Script/Engine.Controller))) "1.000000,1.000000,1.000000") "Undefined" "MultiplyWithRoot" 0 0))
  (Variables|Default|SetCanActivate false)
  (Utilities|FlowControl|Delay (Variables|Default|GetCoolDown))
  (Actor|DestroyActor _returnvalue)
  (Variables|Default|SetCanActivate true))

(event EventBeginPlay)

(event EventTick
  (params (DeltaSeconds :type Float%20%28single-precision%29)))

(fn ActivateAbility
  (if (Variables|Default|GetCanActivate)
    (CallFunction|SpawnShield)
    (|CallParentFunction)))